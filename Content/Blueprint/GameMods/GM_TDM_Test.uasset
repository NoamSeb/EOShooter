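; Test Team Deathmatch game mode in which each death costs the victim's team score, treated as a countdown toward defeat.
; Logins alternate between TeamAlpha and TeamBravo through a FlipFlop on the player state.
; Kills feed UpdateTeamScore, which passes the reduced score to the parent or only prints a game-over message below one.
; BeginPlay sets team lives variables unused elsewhere here, and a deprecated Respawn event forwards to RequestRespawn.
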(event Custom|Respawn
  (params (PlayerController :type BP%20First%20Person%20Player%20Controller%20Object%20Reference))
  ;[1 0 0 0.5] DEPRECATED
  (Class|EOShooterOnlineGameMode|RequestRespawn PlayerController))

(event EventBeginPlay
  (bind _maxteamalive (Variables|Default|GetMaxTeamAlive))
  (bind _returnvalue (+ _maxteamalive 2))
  ;[0.901 0 0.8964 0.5] Default
  (|CallParentFunction)
  (Variables|Default|SetBlueTeamLives _returnvalue)
  (Variables|Default|SetRedTeamLives _returnvalue))

(event EventTick
  (params (DeltaSeconds :type Float%20%28single-precision%29))
  ;[0.901 0 0.8964 0.5] Default
  (|CallParentFunction DeltaSeconds) ; This node is disabled and will not be called.\nDrag off pins to build functionality.
)

(event EventOnPlayerKilled
  (params (Victim :type Controller%20Object%20Reference) (Killer :type Controller%20Object%20Reference))
  ;[0.15 0.15 0.15 0.5] Death Logic
  (Utilities|IsValid Victim
    (:Is%20Valid
      (|CallParentFunction Victim Killer)
      (bind _asonline_player_state (Utilities|Casting|CastToOnlinePlayerState (Variables|/Script/Engine.Controller|GetPlayerState Victim)))
      (Utilities|IsValid _asonline_player_state
        (:Is%20Valid
          (bind _returnvalue (Class|OnlinePlayerState|GetTeam _asonline_player_state))
          (Class|EOShooterOnlineGameMode|UpdateTeamScore _returnvalue 1))
        (:Is%20Not%20Valid
          (Development|PrintString "Game Mod isn't valid"))))
    (:Is%20Not%20Valid
      (Development|PrintString "Victim isn't valid"))))

(event EventPostLogin
  (params (NewPlayer :type Player%20Controller%20Object%20Reference))
  ;[0.15 0.15 0.15 0.5] Post Login
  (|CallParentFunction NewPlayer)
  (bind _asonline_player_state (Utilities|Casting|CastToOnlinePlayerState (Variables|/Script/Engine.Controller|GetPlayerState NewPlayer)))
  (Utilities|FlowControl|FlipFlop
    (:A
      (Class|OnlinePlayerState|SetTeam _asonline_player_state "TeamAlpha"))
    (:B
      (Class|OnlinePlayerState|SetTeam _asonline_player_state "TeamBravo"))))

(event EventUpdateTeamScore
  (params (TeamToUpdate :type ETeamRole%20Enum :default "None") (value :type Integer))
  (bind _teamscores (Variables|Default|GetTeamScores))
  (bind (_value _returnvalue) (Utilities|Map|Find _teamscores TeamToUpdate))
  (bind _returnvalue_2 (- _value value))
  ;[0.15 0.15 0.15 0.5] Death Logic
  ;;[0.15 0.15 0.15 0.5] Score Update
  (if _returnvalue
    (if (< _returnvalue_2 1)
      (Development|PrintString (Utilities|String|Append (Utilities|String|MakeLiteralString "GAME OVER ! ") (Utilities|String|EnumtoString TeamToUpdate) (Utilities|String|MakeLiteralString " LOSE !")))
      (else
        (|CallParentFunction TeamToUpdate _returnvalue_2)))))

(fn ConstructionScript
  (|CallParentFunction))